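; Level editor save/load manager that writes and restores user-built levels through BP_SaveInst save slots.
; On BeginPlay it spawns missing editor actors in a nested check and creates the hidden editor widgets.
; Save captures instanced-mesh transforms for landscape, geometry and foliage, plus lighting, fog, environment materials and spawned activity actors with parameters.
; Load clears instances, refills components by matching mesh, respawns activities, restores the environment, then notifies BI_Input actors.
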(event Custom|Save
  (params (SlotName :type String))
  ;[1 1 1] Save
  (bind _returnvalue (SaveGame|CreateSaveGameObject "/Game/F1LevelEditor/Blueprints/Data/DataComponents/BP_SaveInst.BP_SaveInst_C"))
  (Variables|Default|SetSaveInstance _returnvalue)
  (Utilities|FlowControl|Sequence
    (:then_0
      (Utilities|FlowControl|Sequence
        (:then_0
          ;[1 1 1] Save Landscape
          (bind _outactors (Actor|GetAllActorsOfClass "/Game/F1LevelEditor/Blueprints/Blueprints/BP_ModularLandscape.BP_ModularLandscape_C"))
          (for _array_element (Variables|/Game/F1LevelEditor/Blueprints/Blueprints/BP_ModularLandscape.BP_ModularLandscape_C|GetInstancedComponents (Utilities|Array|Get(acopy) _outactors))
            (Utilities|Array|Clear (Variables|Default|GetBuffer))
            (if (not (<= (Components|InstancedStaticMesh|GetInstanceCount _array_element) 0))
              (for _index (range 0 (Components|InstancedStaticMesh|GetInstanceCount _array_element))
                (Utilities|Array|Add (Variables|Default|GetBuffer) (.OutInstanceTransform (Components|InstancedStaticMesh|GetInstanceTransform _array_element _index true))))
              (Utilities|Array|Add (Variables|/Game/F1LevelEditor/Blueprints/Data/DataComponents/BP_SaveInst.BP_SaveInst_C|GetISM_List (Variables|Default|GetSaveInstance)) (Utilities|Struct|MakeSTR_IsmSave (Variables|Default|GetBuffer) (Variables|/Script/Engine.StaticMeshComponent|GetStaticMesh _array_element) "NewEnumerator0")))))
        (:then_1
          ;[1 1 1] Save Geometry
          (bind _outactors_2 (Actor|GetAllActorsOfClass "/Game/F1LevelEditor/Blueprints/Blueprints/BP_ModularGeometry.BP_ModularGeometry_C"))
          (for _array_element_2 (Variables|/Game/F1LevelEditor/Blueprints/Blueprints/BP_ModularGeometry.BP_ModularGeometry_C|GetInstancedComponents (Utilities|Array|Get(acopy) _outactors_2))
            (Utilities|Array|Clear (Variables|Default|GetBuffer))
            (if (not (<= (Components|InstancedStaticMesh|GetInstanceCount _array_element_2) 0))
              (for _index_2 (range 0 (Components|InstancedStaticMesh|GetInstanceCount _array_element_2))
                (Utilities|Array|Add (Variables|Default|GetBuffer) (.OutInstanceTransform (Components|InstancedStaticMesh|GetInstanceTransform _array_element_2 _index_2 true))))
              (Utilities|Array|Add (Variables|/Game/F1LevelEditor/Blueprints/Data/DataComponents/BP_SaveInst.BP_SaveInst_C|GetISM_List (Variables|Default|GetSaveInstance)) (Utilities|Struct|MakeSTR_IsmSave (Variables|Default|GetBuffer) (Variables|/Script/Engine.StaticMeshComponent|GetStaticMesh _array_element_2) "NewEnumerator1")))))
        (:then_2
          ;[1 1 1] Save Foliage
          (bind _outactors_3 (Actor|GetAllActorsOfClass "/Game/F1LevelEditor/Blueprints/Blueprints/BP_Foliage.BP_Foliage_C"))
          (for _array_element_3 (Variables|/Game/F1LevelEditor/Blueprints/Blueprints/BP_Foliage.BP_Foliage_C|GetInstancedComponents (Utilities|Array|Get(acopy) _outactors_3))
            (Utilities|Array|Clear (Variables|Default|GetBuffer))
            (if (not (<= (Components|InstancedStaticMesh|GetInstanceCount _array_element_3) 0))
              (for _index_3 (range 0 (Components|InstancedStaticMesh|GetInstanceCount _array_element_3))
                (Utilities|Array|Add (Variables|Default|GetBuffer) (.OutInstanceTransform (Components|InstancedStaticMesh|GetInstanceTransform _array_element_3 _index_3 true))))
              (Utilities|Array|Add (Variables|/Game/F1LevelEditor/Blueprints/Data/DataComponents/BP_SaveInst.BP_SaveInst_C|GetISM_List (Variables|Default|GetSaveInstance)) (Utilities|Struct|MakeSTR_IsmSave (Variables|Default|GetBuffer) (Variables|/Script/Engine.StaticMeshComponent|GetStaticMesh _array_element_3) "NewEnumerator2")))))
        (:then_3
          ;[1 1 1] Save Lightning
          (bind _outactors_4 (Actor|GetAllActorsOfClass "/Script/Engine.DirectionalLight"))
          (Variables|Default|SetDL (Utilities|Array|Get(acopy) _outactors_4))
          (bind _outactors_5 (Actor|GetAllActorsOfClass "/Script/Engine.SkyLight"))
          (Variables|Default|SetSL (Utilities|Array|Get(acopy) _outactors_5))
          (bind _outactors_6 (Actor|GetAllActorsOfClass "/Engine/EngineSky/BP_Sky_Sphere.BP_Sky_Sphere_C"))
          (Variables|Default|SetSS (Utilities|Array|Get(acopy) _outactors_6))
          (Variables|/Game/F1LevelEditor/Blueprints/Data/DataComponents/BP_SaveInst.BP_SaveInst_C|SetLightning (Variables|Default|GetSaveInstance) (Utilities|Struct|MakeSTR_LightningInstance (.yaw (Transformation|GetActorRotation (Variables|Default|GetDL))) (.pitch (Transformation|GetActorRotation (Variables|Default|GetDL))) (Variables|/Script/Engine.LightComponentBase|GetIntensity (Variables|/Script/Engine.Light|GetLightComponent (Variables|Default|GetDL))) (Variables|/Script/Engine.LightComponent|GetTemperature (Variables|/Script/Engine.Light|GetLightComponent (Variables|Default|GetDL))) (.r (Rendering|Components|Light|GetLightColor (Variables|/Script/Engine.Light|GetLightComponent (Variables|Default|GetDL)))) (.b (Rendering|Components|Light|GetLightColor (Variables|/Script/Engine.Light|GetLightComponent (Variables|Default|GetDL)))) (.g (Rendering|Components|Light|GetLightColor (Variables|/Script/Engine.Light|GetLightComponent (Variables|Default|GetDL)))) (Variables|/Script/Engine.LightComponentBase|GetIntensity (Variables|/Script/Engine.SkyLight|GetLightComponent (Variables|Default|GetSL))) (.r (Rendering|Components|Light|GetLightColor (Variables|/Script/Engine.SkyLight|GetLightComponent (Variables|Default|GetSL)))) (.b (Rendering|Components|Light|GetLightColor (Variables|/Script/Engine.SkyLight|GetLightComponent (Variables|Default|GetSL)))) (.g (Rendering|Components|Light|GetLightColor (Variables|/Script/Engine.SkyLight|GetLightComponent (Variables|Default|GetSL)))) (Variables|/Engine/EngineSky/BP_Sky_Sphere.BP_Sky_Sphere_C|GetCloud%20opacity (Variables|Default|GetSS)) (Variables|/Engine/EngineSky/BP_Sky_Sphere.BP_Sky_Sphere_C|GetCloud%20speed (Variables|Default|GetSS)) (Variables|/Engine/EngineSky/BP_Sky_Sphere.BP_Sky_Sphere_C|GetStars%20brightness (Variables|Default|GetSS)))))
        (:then_4
          ;[1 1 1] Save Activity
          (bind _foundwidgets (Widget|GetAllWidgetsOfClass "/Game/F1LevelEditor/Blueprints/Widgets/UI_Activity.UI_Activity_C" true))
          (for (_array_element_4 _array_index) (Variables|/Game/F1LevelEditor/Blueprints/Widgets/UI_Activity.UI_Activity_C|GetSpawnedList (Utilities|Array|Get(acopy) _foundwidgets))
            (bind _parameterssctruct (Class|BIInput|GetParametersStructure(Message) (Utilities|Array|Get(acopy) (Variables|/Game/F1LevelEditor/Blueprints/Widgets/UI_Activity.UI_Activity_C|GetSpawnedList_Checker (Utilities|Array|Get(acopy) _foundwidgets)) _array_index)))
            (Utilities|Array|Add (Variables|/Game/F1LevelEditor/Blueprints/Data/DataComponents/BP_SaveInst.BP_SaveInst_C|GetActivity (Variables|Default|GetSaveInstance)) (Utilities|Struct|MakeSTR_SaveActor _array_element_4 (Transformation|GetActorTransform (Utilities|Array|Get(acopy) (Variables|/Game/F1LevelEditor/Blueprints/Widgets/UI_Activity.UI_Activity_C|GetSpawnedList_Checker (Utilities|Array|Get(acopy) _foundwidgets)) _array_index)) (Variables|/Script/Engine.Actor|GetTags (Utilities|Array|Get(acopy) (Variables|/Game/F1LevelEditor/Blueprints/Widgets/UI_Activity.UI_Activity_C|GetSpawnedList_Checker (Utilities|Array|Get(acopy) _foundwidgets)) _array_index)) _parameterssctruct))))
        (:then_5
          ;[1 1 1] Save fog and environment
          (bind _outactors_7 (Actor|GetAllActorsOfClass "/Game/F1LevelEditor/Blueprints/Blueprints/BP_Environment.BP_Environment_C"))
          (Variables|Default|SetEnvironment (Utilities|Array|Get(acopy) _outactors_7))
          (bind _outactors_8 (Actor|GetAllActorsOfClass "/Script/Engine.ExponentialHeightFog"))
          (Variables|/Game/F1LevelEditor/Blueprints/Data/DataComponents/BP_SaveInst.BP_SaveInst_C|SetFogState (Variables|Default|GetSaveInstance) (Utilities|Struct|MakeSTR_FogState (Variables|/Script/Engine.ExponentialHeightFogComponent|GetFogDensity (Variables|/Script/Engine.ExponentialHeightFog|GetComponent (Utilities|Array|Get(acopy) _outactors_8))) (Variables|/Script/Engine.ExponentialHeightFogComponent|GetFogHeightFalloff (Variables|/Script/Engine.ExponentialHeightFog|GetComponent (Utilities|Array|Get(acopy) _outactors_8))) (Variables|/Script/Engine.ExponentialHeightFogComponent|GetFogMaxOpacity (Variables|/Script/Engine.ExponentialHeightFog|GetComponent (Utilities|Array|Get(acopy) _outactors_8))) (Variables|/Script/Engine.ExponentialHeightFogComponent|GetbEnableVolumetricFog (Variables|/Script/Engine.ExponentialHeightFog|GetComponent (Utilities|Array|Get(acopy) _outactors_8)))))
          (Variables|/Game/F1LevelEditor/Blueprints/Data/DataComponents/BP_SaveInst.BP_SaveInst_C|SetBackgroundPanorama (Variables|Default|GetSaveInstance) (Rendering|Material|GetMaterial (Variables|/Game/F1LevelEditor/Blueprints/Blueprints/BP_Environment.BP_Environment_C|GetSkybox (Variables|Default|GetEnvironment)) 0))
          (Variables|/Game/F1LevelEditor/Blueprints/Data/DataComponents/BP_SaveInst.BP_SaveInst_C|SetFloor (Variables|Default|GetSaveInstance) (Rendering|Material|GetMaterial (Variables|/Script/Engine.StaticMeshActor|GetStaticMeshComponent (Variables|Default|GetEnvironment)) 0)))))
    (:then_1
      (SaveGame|SaveGametoSlot (Variables|Default|GetSaveInstance) SlotName)
      (CallFunction|SavetoHeader SlotName))))

(event Custom|Load
  (params (SlotName :type String))
  ;[1 1 1] Load
  (bind _returnvalue (SaveGame|LoadGamefromSlot SlotName))
  (bind _asbp_save_inst (Utilities|Casting|CastToBP_SaveInst _returnvalue)
    (:then
      (bind _output_get (Variables|Default|SetLoadInstance _asbp_save_inst))
      (CallFunction|Clear)
      (for _array_element (Variables|/Game/F1LevelEditor/Blueprints/Data/DataComponents/BP_SaveInst.BP_SaveInst_C|GetISM_List _output_get)
        (Variables|Default|SetCurrentStructure _array_element)
        (switch Utilities|FlowControl|Switch|SwitchonEnum_SaveType (.Type (Utilities|Struct|BreakSTR_IsmSave _array_element))
          (:NewEnumerator0
            ;[0.5459 1 0.332] Load and Use Landscape Datas
            (bind _outactors (Actor|GetAllActorsOfClass "/Game/F1LevelEditor/Blueprints/Blueprints/BP_ModularLandscape.BP_ModularLandscape_C"))
            (for _array_element_2 (Variables|/Game/F1LevelEditor/Blueprints/Blueprints/BP_ModularLandscape.BP_ModularLandscape_C|GetInstancedComponents (Utilities|Array|Get(acopy) _outactors))
              (if (== (Variables|/Script/Engine.StaticMeshComponent|GetStaticMesh _array_element_2) (.object (Variables|Default|GetCurrentStructure)))
                (Components|InstancedStaticMesh|ClearInstances _array_element_2)
                (for _array_element_3 (.locations (Variables|Default|GetCurrentStructure))
                  (Class|InstancedStaticMeshComponent|AddInstanceWorldSpace _array_element_2 _array_element_3)))))
          (:NewEnumerator1
            ;[0.5194 0.7605 1] Load and Use Geometry Datas
            (bind _outactors_2 (Actor|GetAllActorsOfClass "/Game/F1LevelEditor/Blueprints/Blueprints/BP_ModularGeometry.BP_ModularGeometry_C"))
            (for _array_element_4 (Variables|/Game/F1LevelEditor/Blueprints/Blueprints/BP_ModularGeometry.BP_ModularGeometry_C|GetInstancedComponents (Utilities|Array|Get(acopy) _outactors_2))
              (if (== (Variables|/Script/Engine.StaticMeshComponent|GetStaticMesh _array_element_4) (.object (Variables|Default|GetCurrentStructure)))
                (Components|InstancedStaticMesh|ClearInstances _array_element_4)
                (for _array_element_5 (.locations (Variables|Default|GetCurrentStructure))
                  (Class|InstancedStaticMeshComponent|AddInstanceWorldSpace _array_element_4 _array_element_5)))))
          (:NewEnumerator2
            ;[1 0.4612 0.3914] Load and Use Foliage Datas
            (bind _outactors_3 (Actor|GetAllActorsOfClass "/Game/F1LevelEditor/Blueprints/Blueprints/BP_Foliage.BP_Foliage_C"))
            (for _array_element_6 (Variables|/Game/F1LevelEditor/Blueprints/Blueprints/BP_Foliage.BP_Foliage_C|GetInstancedComponents (Utilities|Array|Get(acopy) _outactors_3))
              (if (== (Variables|/Script/Engine.StaticMeshComponent|GetStaticMesh _array_element_6) (.object (Variables|Default|GetCurrentStructure)))
                (Components|InstancedStaticMesh|ClearInstances _array_element_6)
                (for _array_element_7 (.locations (Variables|Default|GetCurrentStructure))
                  (Class|InstancedStaticMeshComponent|AddInstanceWorldSpace _array_element_6 _array_element_7)))))))
      (Utilities|FlowControl|Sequence
        (:then_0
          ;[1 1 1] Lightning Load
          (bind _outactors_4 (Actor|GetAllActorsOfClass "/Script/Engine.DirectionalLight"))
          (Variables|Default|SetDL (Utilities|Array|Get(acopy) _outactors_4))
          (bind _outactors_5 (Actor|GetAllActorsOfClass "/Script/Engine.SkyLight"))
          (Variables|Default|SetSL (Utilities|Array|Get(acopy) _outactors_5))
          (bind _outactors_6 (Actor|GetAllActorsOfClass "/Engine/EngineSky/BP_Sky_Sphere.BP_Sky_Sphere_C"))
          (Variables|Default|SetSS (Utilities|Array|Get(acopy) _outactors_6))
          (Transformation|SetActorRotation (Variables|Default|GetDL) (Math|Rotator|MakeRotator 0.0 (.dl_vertical (Variables|/Game/F1LevelEditor/Blueprints/Data/DataComponents/BP_SaveInst.BP_SaveInst_C|GetLightning (Variables|Default|GetLoadInstance))) (.dl_horizontal (Variables|/Game/F1LevelEditor/Blueprints/Data/DataComponents/BP_SaveInst.BP_SaveInst_C|GetLightning (Variables|Default|GetLoadInstance)))))
          (Rendering|Components|Light|SetIntensity (Variables|/Script/Engine.Light|GetLightComponent (Variables|Default|GetDL)) (.dl_intensity (Variables|/Game/F1LevelEditor/Blueprints/Data/DataComponents/BP_SaveInst.BP_SaveInst_C|GetLightning (Variables|Default|GetLoadInstance))))
          (Class|LightComponent|SetTemperature (Variables|/Script/Engine.Light|GetLightComponent (Variables|Default|GetDL)) (.dl_temperature (Variables|/Game/F1LevelEditor/Blueprints/Data/DataComponents/BP_SaveInst.BP_SaveInst_C|GetLightning (Variables|Default|GetLoadInstance))))
          (Rendering|Components|Light|SetLightColor (Variables|/Script/Engine.Light|GetLightComponent (Variables|Default|GetDL)) (Utilities|Struct|MakeLinearColor (.dl_red (Variables|/Game/F1LevelEditor/Blueprints/Data/DataComponents/BP_SaveInst.BP_SaveInst_C|GetLightning (Variables|Default|GetLoadInstance))) (.dl_green (Variables|/Game/F1LevelEditor/Blueprints/Data/DataComponents/BP_SaveInst.BP_SaveInst_C|GetLightning (Variables|Default|GetLoadInstance))) (.dl_blue (Variables|/Game/F1LevelEditor/Blueprints/Data/DataComponents/BP_SaveInst.BP_SaveInst_C|GetLightning (Variables|Default|GetLoadInstance))) 1.0) true)
          (Rendering|Components|Light|SetIntensity (Variables|/Script/Engine.SkyLight|GetLightComponent (Variables|Default|GetSL)) (.sl_intensity (Variables|/Game/F1LevelEditor/Blueprints/Data/DataComponents/BP_SaveInst.BP_SaveInst_C|GetLightning (Variables|Default|GetLoadInstance))))
          (Rendering|Components|Light|SetLightColor (Variables|/Script/Engine.SkyLight|GetLightComponent (Variables|Default|GetSL)) (Utilities|Struct|MakeLinearColor (.sl_red (Variables|/Game/F1LevelEditor/Blueprints/Data/DataComponents/BP_SaveInst.BP_SaveInst_C|GetLightning (Variables|Default|GetLoadInstance))) (.sl_green (Variables|/Game/F1LevelEditor/Blueprints/Data/DataComponents/BP_SaveInst.BP_SaveInst_C|GetLightning (Variables|Default|GetLoadInstance))) (.sl_blue (Variables|/Game/F1LevelEditor/Blueprints/Data/DataComponents/BP_SaveInst.BP_SaveInst_C|GetLightning (Variables|Default|GetLoadInstance))) 1.0))
          (Variables|/Engine/EngineSky/BP_Sky_Sphere.BP_Sky_Sphere_C|SetCloud%20opacity (Variables|Default|GetSS) (.c_cloudopacity (Variables|/Game/F1LevelEditor/Blueprints/Data/DataComponents/BP_SaveInst.BP_SaveInst_C|GetLightning (Variables|Default|GetLoadInstance))))
          (Variables|/Engine/EngineSky/BP_Sky_Sphere.BP_Sky_Sphere_C|SetCloud%20speed (Variables|Default|GetSS) (.c_cloudspeed (Variables|/Game/F1LevelEditor/Blueprints/Data/DataComponents/BP_SaveInst.BP_SaveInst_C|GetLightning (Variables|Default|GetLoadInstance))))
          (Variables|/Engine/EngineSky/BP_Sky_Sphere.BP_Sky_Sphere_C|SetStars%20brightness (Variables|Default|GetSS) (.c_starsopacity (Variables|/Game/F1LevelEditor/Blueprints/Data/DataComponents/BP_SaveInst.BP_SaveInst_C|GetLightning (Variables|Default|GetLoadInstance))))
          (Default|RefreshMaterial (Variables|Default|GetSS))
          (Class|SkyLightComponent|RecaptureSky (Variables|/Script/Engine.SkyLight|GetLightComponent (Variables|Default|GetSL))))
        (:then_1
          ;[1 1 1] Activity Load
          (bind _foundwidgets (Widget|GetAllWidgetsOfClass "/Game/F1LevelEditor/Blueprints/Widgets/UI_Activity.UI_Activity_C" true))
          (for _array_element_8 (Variables|/Game/F1LevelEditor/Blueprints/Widgets/UI_Activity.UI_Activity_C|GetSpawnedList_Checker (Utilities|Array|Get(acopy) _foundwidgets))
            (Utilities|IsValid _array_element_8
              (:Is%20Valid
                (Actor|DestroyActor _array_element_8))))
          (Utilities|Array|Clear (Variables|/Game/F1LevelEditor/Blueprints/Widgets/UI_Activity.UI_Activity_C|GetSpawnedList_Checker (Utilities|Array|Get(acopy) _foundwidgets)))
          (Utilities|Array|Clear (Variables|/Game/F1LevelEditor/Blueprints/Widgets/UI_Activity.UI_Activity_C|GetSpawnedList (Utilities|Array|Get(acopy) _foundwidgets)))
          (for _array_element_9 (Variables|/Game/F1LevelEditor/Blueprints/Data/DataComponents/BP_SaveInst.BP_SaveInst_C|GetActivity (Variables|Default|GetLoadInstance))
            (bind _returnvalue_2 (Game|SpawnActorfromClass (.actor _array_element_9) (.transform _array_element_9) "Undefined" 0 0))
            (Utilities|Array|Add (Variables|/Game/F1LevelEditor/Blueprints/Widgets/UI_Activity.UI_Activity_C|GetSpawnedList_Checker (Utilities|Array|Get(acopy) _foundwidgets)) _returnvalue_2)
            (Utilities|Array|Add (Variables|/Game/F1LevelEditor/Blueprints/Widgets/UI_Activity.UI_Activity_C|GetSpawnedList (Utilities|Array|Get(acopy) _foundwidgets)) (Utilities|GetClass _returnvalue_2))
            (Variables|/Script/Engine.Actor|SetTags _returnvalue_2 (.tagsarr _array_element_9))
            (Class|BIInput|Loaded(Message) _returnvalue_2 (.parameters _array_element_9))))
        (:then_2
          ;[1 1 1] Fog and environment load
          (bind _outactors_7 (Actor|GetAllActorsOfClass "/Game/F1LevelEditor/Blueprints/Blueprints/BP_Environment.BP_Environment_C"))
          (Variables|Default|SetEnvironment (Utilities|Array|Get(acopy) _outactors_7))
          (Utilities|FlowControl|Sequence
            (:then_0
              (bind _outactors_8 (Actor|GetAllActorsOfClass "/Script/Engine.ExponentialHeightFog"))
              (Class|ExponentialHeightFogComponent|SetFogDensity (Variables|/Script/Engine.ExponentialHeightFog|GetComponent (Utilities|Array|Get(acopy) _outactors_8)) (.density (Variables|/Game/F1LevelEditor/Blueprints/Data/DataComponents/BP_SaveInst.BP_SaveInst_C|GetFogState (Variables|Default|GetLoadInstance))))
              (Class|ExponentialHeightFogComponent|SetFogHeightFalloff (Variables|/Script/Engine.ExponentialHeightFog|GetComponent (Utilities|Array|Get(acopy) _outactors_8)) (.falloff (Variables|/Game/F1LevelEditor/Blueprints/Data/DataComponents/BP_SaveInst.BP_SaveInst_C|GetFogState (Variables|Default|GetLoadInstance))))
              (Class|ExponentialHeightFogComponent|SetFogMaxOpacity (Variables|/Script/Engine.ExponentialHeightFog|GetComponent (Utilities|Array|Get(acopy) _outactors_8)) (.maxopacity (Variables|/Game/F1LevelEditor/Blueprints/Data/DataComponents/BP_SaveInst.BP_SaveInst_C|GetFogState (Variables|Default|GetLoadInstance))))
              (Class|ExponentialHeightFogComponent|SetVolumetricFog (Variables|/Script/Engine.ExponentialHeightFog|GetComponent (Utilities|Array|Get(acopy) _outactors_8)) (.isvolumetric (Variables|/Game/F1LevelEditor/Blueprints/Data/DataComponents/BP_SaveInst.BP_SaveInst_C|GetFogState (Variables|Default|GetLoadInstance)))))
            (:then_1
              (Rendering|Material|SetMaterial (Variables|/Game/F1LevelEditor/Blueprints/Blueprints/BP_Environment.BP_Environment_C|GetSkybox (Variables|Default|GetEnvironment)) 0 (Variables|/Game/F1LevelEditor/Blueprints/Data/DataComponents/BP_SaveInst.BP_SaveInst_C|GetBackgroundPanorama (Variables|Default|GetLoadInstance)))
              (Rendering|Material|SetMaterial (Variables|/Script/Engine.StaticMeshActor|GetStaticMeshComponent (Variables|Default|GetEnvironment)) 0 (Variables|/Game/F1LevelEditor/Blueprints/Data/DataComponents/BP_SaveInst.BP_SaveInst_C|GetFloor (Variables|Default|GetLoadInstance)))
              (bind _foundwidgets_2 (Widget|GetAllWidgetsOfClass "/Game/F1LevelEditor/Blueprints/Widgets/UI_LighningEditor.UI_LighningEditor_C" true))
              (Class|ComboBoxString|SetSelectedOption (Variables|/Game/F1LevelEditor/Blueprints/Widgets/UI_LighningEditor.UI_LighningEditor_C|GetCB_FloorMat (Utilities|Array|Get(acopy) _foundwidgets_2)) (Utilities|GetDisplayName (Variables|/Game/F1LevelEditor/Blueprints/Data/DataComponents/BP_SaveInst.BP_SaveInst_C|GetFloor (Variables|Default|GetLoadInstance)))) ; Unselect options in widget
              (Class|ComboBoxString|SetSelectedOption (Variables|/Game/F1LevelEditor/Blueprints/Widgets/UI_LighningEditor.UI_LighningEditor_C|GetCB_Panorama (Utilities|Array|Get(acopy) _foundwidgets_2)) (Utilities|GetDisplayName (Variables|/Game/F1LevelEditor/Blueprints/Data/DataComponents/BP_SaveInst.BP_SaveInst_C|GetBackgroundPanorama (Variables|Default|GetLoadInstance)))) ; Unselect options in widget
            )))
        (:then_3
          ;[0.8274 0.2517 1] Notice activity, when load is complete
          (bind _outactors_9 (Actor|GetAllActorswithInterface "/Game/F1LevelEditor/Blueprints/Data/DataComponents/BI_Input.BI_Input_C"))
          (for _array_element_10 _outactors_9
            (Class|BIInput|AllActivityLoaded(Message) _array_element_10)))))
    (:CastFailed
      ;[1 0.2322 0.09237] [DEBUG] Save not found
      (Development|PrintString "Save file doesnt exist or damaged" true true "(R=0.000000,G=0.660000,B=1.000000,A=1.000000)" 5.0))))

(event Custom|Clear
  ;[1 1 1] Clear level before load
  (bind _outactors (Actor|GetAllActorsOfClass "/Game/F1LevelEditor/Blueprints/Blueprints/BP_ModularLandscape.BP_ModularLandscape_C"))
  (for _array_element (Variables|/Game/F1LevelEditor/Blueprints/Blueprints/BP_ModularLandscape.BP_ModularLandscape_C|GetInstancedComponents (Utilities|Array|Get(acopy) _outactors))
    (Components|InstancedStaticMesh|ClearInstances _array_element))
  (bind _outactors_2 (Actor|GetAllActorsOfClass "/Game/F1LevelEditor/Blueprints/Blueprints/BP_ModularGeometry.BP_ModularGeometry_C"))
  (for _array_element_2 (Variables|/Game/F1LevelEditor/Blueprints/Blueprints/BP_ModularGeometry.BP_ModularGeometry_C|GetInstancedComponents (Utilities|Array|Get(acopy) _outactors_2))
    (Components|InstancedStaticMesh|ClearInstances _array_element_2))
  (bind _outactors_3 (Actor|GetAllActorsOfClass "/Game/F1LevelEditor/Blueprints/Blueprints/BP_Foliage.BP_Foliage_C"))
  (for _array_element_3 (Variables|/Game/F1LevelEditor/Blueprints/Blueprints/BP_Foliage.BP_Foliage_C|GetInstancedComponents (Utilities|Array|Get(acopy) _outactors_3))
    (Components|InstancedStaticMesh|ClearInstances _array_element_3)))

(event EventBeginPlay
  ;[1 1 1] Preset
  (Utilities|FlowControl|Sequence
    (:then_0
      (bind _is_valid (CallFunction|GetLandscapeBP))
      (if (not _is_valid)
        (Game|SpawnActorfromClass "/Game/F1LevelEditor/Blueprints/Blueprints/BP_ModularLandscape.BP_ModularLandscape_C" (Math|Transform|MakeTransform "0, 0, 0" "0, 0, 0" "1,1,1") "Undefined" 0 0)
        (bind _is_valid_2 (CallFunction|GetFoliageBP))
        (if (not _is_valid_2)
          (Game|SpawnActorfromClass "/Game/F1LevelEditor/Blueprints/Blueprints/BP_Foliage.BP_Foliage_C" (Math|Transform|MakeTransform "0, 0, 0" "0, 0, 0" "1,1,1") "Undefined" 0 0)
          (bind _is_valid_3 (CallFunction|GetGeometryBP))
          (if (not _is_valid_3)
            (Game|SpawnActorfromClass "/Game/F1LevelEditor/Blueprints/Blueprints/BP_ModularGeometry.BP_ModularGeometry_C" (Math|Transform|MakeTransform "0, 0, 0" "0, 0, 0" "1,1,1") "Undefined" 0 0)
            (bind _is_valid_4 (CallFunction|GetActivityBP))
            (if (not _is_valid_4)
              (Game|SpawnActorfromClass "/Game/F1LevelEditor/Blueprints/Blueprints/BP_Activity.BP_Activity_C" (Math|Transform|MakeTransform "0, 0, 0" "0, 0, 0" "1,1,1") "Undefined" 0 0))))))
    (:then_1
      (bind _returnvalue (UserInterface|CreateWidget "/Game/F1LevelEditor/Blueprints/Widgets/UI_ModularGeometry.UI_ModularGeometry_C"))
      (bind _returnvalue_2 (UserInterface|CreateWidget "/Game/F1LevelEditor/Blueprints/Widgets/UI_FoliageEditor.UI_FoliageEditor_C"))
      (bind _returnvalue_3 (UserInterface|CreateWidget "/Game/F1LevelEditor/Blueprints/Widgets/UI_LandscapeEditor.UI_LandscapeEditor_C"))
      (bind _returnvalue_4 (UserInterface|CreateWidget "/Game/F1LevelEditor/Blueprints/Widgets/UI_Activity.UI_Activity_C"))
      (UserInterface|Viewport|AddtoViewport _returnvalue_2 0)
      (Widget|SetVisibility _returnvalue_2 "Hidden"))
    (:then_2
      (CallFunction|DisableAllTooltips))))

(fn ConstructionScript)