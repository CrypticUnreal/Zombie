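; Level-editor example activity: a clickable button that sends a turn-on message to other actors linked by tag.
; The target tag is exposed as a parameter, and tagged actors are cached once all activities load.
; With the player nearby, Tick polls a key and traces for a button to press.
; A press turns the dynamic material red, messages targets and blocks re-pressing until a delay restores grey, without sending an off message.
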(event Custom|on
  (if (Variables|Default|GetCanPress?)
    (Rendering|Material|SetVectorParameterValue (Variables|Default|GetMaterial) "Color" "(R=1.000000,G=0.000000,B=0.000000,A=1.000000)" :!class /Script/Engine.MaterialInstanceDynamic)
    (Utilities|FlowControl|Sequence
      (:then_0
        (Variables|Default|SetCanPress? false)
        (for _array_element (Variables|Settings|GetOutput%20to:)
          (Class|BIInput|InputTurn(Message) _array_element true)))
      (:then_1
        (Utilities|FlowControl|Delay (Variables|Settings|GetTurnOnDelay))
        (Rendering|Material|SetVectorParameterValue (Variables|Default|GetMaterial) "Color" "(R=0.300000,G=0.300000,B=0.300000,A=1.000000)" :!class /Script/Engine.MaterialInstanceDynamic) ; Change color then off
        (Variables|Default|SetCanPress? true)))))

(event EventTick
  (params (DeltaSeconds :type Float%20%28single-precision%29))
  (bind _is_near (CallFunction|ActorIsNear self 5e+02))
  (if _is_near
    (if (Game|Player|IsInputKeyDown (Game|GetPlayerController 0) (Variables|Settings|GetKey))
      (bind _hitactor (CallFunction|TracefromActor (Variables|Default|GetDistantionForPress) false (Utilities|Array|MakeArray (Game|Player|GetPlayerPawn 0)) false "TraceTypeQuery1"))
      (bind _asbp_click_button (Utilities|Casting|CastToBP_Example_ClickButton _hitactor))
      (CallFunction|On _asbp_click_button))))

(event EventLoaded
  (params (Params :type STR%20Parameters%20Save%20Structure))
  (Variables|Default|SetTagsPoint (Utilities|Struct|BreakSTR_ParametersSave Params)))

(event EventAllActivityLoaded
  (bind _outactors (Actor|GetAllActorswithTag (Variables|Default|GetTagsPoint)))
  (Variables|Settings|SetOutput%20to: _outactors))

(fn ConstructionScript
  (bind _returnvalue (Rendering|Material|CreateDynamicMaterialInstance "/Game/F1LevelEditor/Materials/Instance/MI_ClickButton.MI_ClickButton" "None" :!class /Script/Engine.KismetMaterialLibrary))
  (bind _output_get (Variables|Default|SetMaterial _returnvalue))
  (Rendering|Material|SetMaterial (Variables|Default|GetStaticMesh) 1 _output_get))

(fn GetParametersStructure
  (return (Utilities|Struct|MakeSTR_ParametersSave (Variables|Default|GetTagsPoint))))