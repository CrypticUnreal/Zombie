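; BP_Example_Door is an example double sliding door for the level editor's activity Blueprints, opened and closed by a boolean turn input.
; InputTurn calls Open or Close, which play or reverse a single timeline.
; The timeline track slides the Right and Left components apart symmetrically along relative X at a fixed height.
; GetParametersStructure is an empty stub, so the door supplies no parameters.
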(event Custom|Open
  (bind _track (Timeline|TL_Open Play)
    (:Update
      (Transformation|SetRelativeLocation (Variables|Default|GetRight) (Math|Vector|MakeVector (+ _track 1e+02) 0.0 2e+02) false false)
      (Transformation|SetRelativeLocation (Variables|Default|GetLeft) (Math|Vector|MakeVector (- (* _track -1.0) 1e+02) 0.0 2e+02) false false))))

(event Custom|Close
  (bind _track (Timeline|TL_Open Reverse)
    (:Update
      (Transformation|SetRelativeLocation (Variables|Default|GetRight) (Math|Vector|MakeVector (+ _track 1e+02) 0.0 2e+02) false false)
      (Transformation|SetRelativeLocation (Variables|Default|GetLeft) (Math|Vector|MakeVector (- (* _track -1.0) 1e+02) 0.0 2e+02) false false))))

(event EventInputTurn
  (params (Turn :type Boolean))
  (if Turn
    (CallFunction|Open)
    (else
      (CallFunction|Close))))

(fn ConstructionScript)

(fn GetParametersStructure
  (return ""))