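; BP_ModularLandscape is the level editor's build surface, where blocks are placed and removed on a configurable grid.
; The UI supplies entries that each become an instanced static mesh component, paired with an enum that selects the active brush.
; Spawning adds grid-snapped instances to that brush's component, while a green tooltip mesh previews placement.
; The floor is one mesh scaled to X/Y counts rather than instanced tiles, for performance.
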(event Custom|ShowTooltip
  (params (Directed%20Location :type Vector))
  ;[1 1 1] Tooltips
  (Transformation|SetWorldTransform (Variables|Default|GetEditorTooltip) (Math|Transform|MakeTransform (Class|KismetMathLibrary|VectorSnappedtoGrid Directed%20Location (Variables|Default|GetCONFIG_GrindScale)) (Variables|Default|GetMeshRot) (Variables|Default|GetScaleT)) false true))

(event Custom|Destroy%20Item
  (params (InstanceIndex :type Integer) (Component :type Actor%20Component%20Object%20Reference))
  ;[1 1 1] Destroy Block
  (bind _asinstanced_static_mesh_component (Utilities|Casting|CastToInstancedStaticMeshComponent Component))
  (Class|InstancedStaticMeshComponent|RemoveInstance _asinstanced_static_mesh_component InstanceIndex))

(event Custom|Generate
  (params (X%20count :type Integer) (Y%20count :type Integer))
  ;[0.1731 0.3594 0] Generate Floor with XY counts. We doesnt generate instance floor for optimize. Ocean will hide floor
  (bind _output_get (Variables|Default|SetY Y%20count))
  (bind _output_get_2 (Variables|Default|SetX X%20count))
  (Transformation|SetRelativeScale3D (Variables|Default|GetStaticMesh) (Math|Vector|MakeVector (Math|Conversions|ToFloat(Integer) _output_get_2) (Math|Conversions|ToFloat(Integer) _output_get) 0.0)))

(event Custom|Spawn%20Item
  (params (InstanceIndex :type Integer) (Component :type Actor%20Component%20Object%20Reference) (Location :type Vector) (DirectedLoc :type Vector))
  ;[1 1 1] Spawn Item
  (if (== Component (Utilities|Array|Get(acopy) (Variables|Default|GetInstancedComponents))) ; If true, spawn upper
    (Components|InstancedStaticMesh|AddInstance (Variables|Default|GetCurrentSpawnType) (Math|Transform|MakeTransform (Class|KismetMathLibrary|VectorSnappedtoGrid DirectedLoc (Variables|Default|GetCONFIG_GrindScale)) (Variables|Default|GetMeshRot) (Variables|Default|GetScaleT)))
    (elif (== Component (Variables|Default|GetStaticMesh))
      (Class|InstancedStaticMeshComponent|AddInstanceWorldSpace (Variables|Default|GetCurrentSpawnType) (Math|Transform|MakeTransform (Class|KismetMathLibrary|VectorSnappedtoGrid Location (Variables|Default|GetCONFIG_GrindScale)) (Variables|Default|GetMeshRot) (Variables|Default|GetScaleT))))))

(event Custom|ChangeBrush
  (params (Type :type Enum_LandscapeTypes%20Enum%20%28by%20ref%29 :default "NewEnumerator0"))
  (bind _editortooltip (Variables|Default|GetEditorTooltip))
  ;[1 0.2181 0.05805] Change current brush. Called from UI with enum type.
  (bind _output_get (Variables|Default|SetCurrentSpawnType (Utilities|Array|Get(acopy) (Variables|Default|GetInstancedComponents) (Utilities|Array|FindItem (Variables|Default|GetEnumComp) Type))))
  (Components|StaticMesh|SetStaticMesh (Variables|Default|GetEditorTooltip) (Variables|/Script/Engine.StaticMeshComponent|GetStaticMesh _output_get))
  ;[1 1 1] Change Materials to green in tooltip
  (for _index (range 0 (Rendering|Material|GetNumMaterials _editortooltip))
    (Rendering|Material|SetMaterial _editortooltip _index "/Game/F1LevelEditor/Materials/Instance/MI_True.MI_True")))

(event Custom|GenerateFromUI
  (params (NewParam :type Array%20of%20STR%20Landscape%20Structures))
  ;[1 0.1073 0.02767] Generate instanced meshes for each object in data table. Called from UI with structure input.
  (for _array_element NewParam
    (bind _returnvalue (AddComponent|AddInstancedStaticMeshComponent true))
    (Components|StaticMesh|SetStaticMesh _returnvalue (.Staticmesh (Utilities|Struct|BreakSTR_Landscape _array_element)))
    (Utilities|Array|Add (Variables|Default|GetInstancedComponents) _returnvalue)
    (Utilities|Array|Add (Variables|Default|GetEnumComp) (.Nameinenum (Utilities|Struct|BreakSTR_Landscape _array_element)))
    (for (_array_element_2 _array_index) (.OverrideMaterialOptional (Utilities|Struct|BreakSTR_Landscape _array_element))
      (Rendering|Material|SetMaterial _returnvalue _array_index _array_element_2)))
  (CallFunction|StartupSelect))

(event Custom|StartupSelect
  ;[0.5872 1 0] Select first element on start. Else this be clear and call errors
  (Variables|Default|SetCurrentSpawnType (Utilities|Array|Get(acopy) (Variables|Default|GetInstancedComponents))))

(event EventBeginPlay
  ;[1 1 1] Load Config
  (bind _gridscale (CallFunction|GetConfig))
  (Variables|Default|SetCONFIG_GrindScale _gridscale))

(fn ConstructionScript)