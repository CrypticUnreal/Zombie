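; BP_ModularGeometry is the level editor's block placer, managing modular geometry as instanced static meshes.
; Generate builds one instanced mesh component per UI-supplied entry, with optional material overrides, indexed through a parallel enum array.
; ChangeBrush picks the active component, SpawnItem adds grid-snapped instances to it, and DestroyItem removes instances by index.
; A tooltip mesh previews the current brush at the snapped location, using the grid scale from config.
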(event Custom|ShowTooltip
  (params (Directed%20Location :type Vector))
  ;[1 1 1] Tooltips
  (Transformation|SetWorldTransform (Variables|Default|GetTooltipM) (Math|Transform|MakeTransform (Class|KismetMathLibrary|VectorSnappedtoGrid Directed%20Location (Variables|Default|GetCONFIG_GridScale)) (Variables|Default|GetMeshRot) (Variables|Default|GetScaleT)) false true))

(event Custom|Destroy%20Item
  (params (InstanceIndex :type Integer) (Component :type Actor%20Component%20Object%20Reference))
  ;[1 1 1] Destroy Block
  (bind _asinstanced_static_mesh_component (Utilities|Casting|CastToInstancedStaticMeshComponent Component))
  (Class|InstancedStaticMeshComponent|RemoveInstance _asinstanced_static_mesh_component InstanceIndex))

(event Custom|Spawn%20Item
  (params (DirectedLoc :type Vector))
  ;[1 1 1] Spawn Item
  (Components|InstancedStaticMesh|AddInstance (Variables|Default|GetCurrentSpawnType) (Math|Transform|MakeTransform (Class|KismetMathLibrary|VectorSnappedtoGrid DirectedLoc (Variables|Default|GetCONFIG_GridScale)) (Variables|Default|GetMeshRot) (Variables|Default|GetScaleT))))

(event Custom|ChangeBrush
  (params (Type :type Enum_GeometryTypes%20Enum :default "NewEnumerator0"))
  ;[1 0.2181 0.05805] Change current brush. Called from UI with enum type.
  (bind _output_get (Variables|Default|SetCurrentSpawnType (Utilities|Array|Get(acopy) (Variables|Default|GetInstancedComponents) (Utilities|Array|FindItem (Variables|Default|GetEnumComponents) Type))))
  (Components|StaticMesh|SetStaticMesh (Variables|Default|GetTooltipM) (Variables|/Script/Engine.StaticMeshComponent|GetStaticMesh _output_get)))

(event Custom|Generate
  (params (In%20Structure :type Array%20of%20STR%20Geometry%20Structures))
  ;[1 0.1073 0.02767] Generate instanced meshes for each object in data table. Called from UI with structure input.
  (for _array_element In%20Structure
    (bind _returnvalue (AddComponent|AddInstancedStaticMeshComponent true))
    (Components|StaticMesh|SetStaticMesh _returnvalue (.Staticmesh (Utilities|Struct|BreakSTR_Geometry _array_element)))
    (Utilities|Array|Add (Variables|Default|GetInstancedComponents) _returnvalue)
    (Utilities|Array|Add (Variables|Default|GetEnumComponents) (.Nameinenum (Utilities|Struct|BreakSTR_Geometry _array_element)))
    (for (_array_element_2 _array_index) (.OverrideMaterialOptional (Utilities|Struct|BreakSTR_Geometry _array_element))
      (Rendering|Material|SetMaterial _returnvalue _array_index _array_element_2)))
  (CallFunction|StartupSelect))

(event Custom|StartupSelect
  ;[0.5872 1 0] Select first element on start. Else this be clear and call errors
  (Variables|Default|SetCurrentSpawnType (Utilities|Array|Get(acopy) (Variables|Default|GetInstancedComponents))))

(event EventBeginPlay
  ;[1 1 1] Load Config
  (bind _gridscale (CallFunction|GetConfig))
  (Variables|Default|SetCONFIG_GridScale _gridscale))

(fn ConstructionScript)