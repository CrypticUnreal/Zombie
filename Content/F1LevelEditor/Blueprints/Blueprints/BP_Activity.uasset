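; BP_Activity manages brush selection and a preview mesh for actor types in the level editor.
; Generate fills parallel class, enum, widget and mesh arrays from UI-supplied data, falling back to a sphere mesh, and selects the first class.
; ChangeBrush looks up the enum's index to set the current class, widget and tooltip mesh.
; The tooltip uses MI_True on its materials and teleports to given locations with a pivot shift and rotation.
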(event Custom|Generate
  (params (NewParam :type Array%20of%20STR%20Activity%20Structures))
  ;[1 0.1073 0.02767] Generate instanced meshes for each object in data table. Called from UI with structure input.
  (for _array_element NewParam
    (Utilities|Array|Add (Variables|Default|GetClass%20Array) (.Actor (Utilities|Struct|BreakSTR_Activity _array_element)))
    (Utilities|Array|Add (Variables|Default|GetEnumComponents) (.Nameinenum (Utilities|Struct|BreakSTR_Activity _array_element)))
    (Utilities|Array|Add (Variables|Default|GetWidgetsClass) (.ParameterspickerwidgetOptional (Utilities|Struct|BreakSTR_Activity _array_element)))
    (Utilities|IsValid (.PreviewMeshOptional (Utilities|Struct|BreakSTR_Activity _array_element))
      (:Is%20Valid
        (Utilities|Array|Add (Variables|Default|GetMeshes) (.PreviewMeshOptional (Utilities|Struct|BreakSTR_Activity _array_element))))
      (:Is%20Not%20Valid
        (Utilities|Array|Add (Variables|Default|GetMeshes) "/Game/F1LevelEditor/Meshes/SM_FoliageSphere.SM_FoliageSphere"))))
  (CallFunction|StartupSelect))

(event Custom|Change%20Tooltip
  (params (NewParam :type Static%20Mesh%20Object%20Reference))
  (bind _tooltip (Variables|Default|GetTooltip))
  ;[1 0.736 0] Tooltips
  (Components|StaticMesh|SetStaticMesh _tooltip NewParam)
  (for _index (range 0 (Rendering|Material|GetNumMaterials _tooltip))
    (Rendering|Material|SetMaterial (Variables|Default|GetTooltip) _index "/Game/F1LevelEditor/Materials/Instance/MI_True.MI_True")))

(event Custom|ShowAndMoveToolTip
  (params (NewLocation :type Vector) (PivotShift :type Vector) (NewRotation :type Rotator))
  (bind _tooltip (Variables|Default|GetTooltip))
  ;[1 0.736 0] Tooltips
  (Transformation|SetWorldLocation _tooltip (+ NewLocation PivotShift) false true)
  (Transformation|SetWorldRotation _tooltip NewRotation false false))

(event Custom|ChangeBrush
  (params (Type :type Enum_Activity%20Enum :default "NewEnumerator5"))
  (bind _enumcomponents (Variables|Default|GetEnumComponents))
  (bind _returnvalue (Utilities|Array|FindItem _enumcomponents Type))
  ;[1 0.2181 0.05805] Change current brush. Called from UI with enum type.
  (Variables|Default|SetCurrent%20Class (Utilities|Array|Get(acopy) (Variables|Default|GetClass%20Array) _returnvalue))
  (CallFunction|ChangeTooltip (Utilities|Array|Get(acopy) (Variables|Default|GetMeshes) _returnvalue))
  (Variables|Default|SetCurrentWidget (Utilities|Array|Get(acopy) (Variables|Default|GetWidgetsClass) _returnvalue)))

(event Custom|StartupSelect
  ;[0.5872 1 0] Select first element on start.
  (Variables|Default|SetCurrent%20Class (Utilities|Array|Get(acopy) (Variables|Default|GetClass%20Array))))

(fn ConstructionScript)